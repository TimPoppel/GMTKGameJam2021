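; A spider den variant of a web slot that becomes claimed when a web connects and spawns a spider while claimed.
; Connecting a web spawns the spider at the Arrow's transform, and web removal destroys it and clears the claim once no web remains.
; Cube materials show hover and claimed states, while click, deselect and removal events extend the parent slot's behavior.
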(event OnBeginCursorOver(Cube)
  (params (TouchedComponent :type Primitive%20Component%20Object%20Reference))
  (if (not (Variables|Default|GetIsSelected))
    (Rendering|Material|SetMaterial (Variables|Default|GetCube) 0 "/DatasmithContent/Materials/Arealight.Arealight")))

(event OnEndCursorOver(Cube)
  (params (TouchedComponent :type Primitive%20Component%20Object%20Reference))
  (bind _cube (Variables|Default|GetCube))
  (if (not (Variables|Default|GetIsSelected))
    (if (Variables|Default|GetIsClaimed)
      (Rendering|Material|SetMaterial _cube 0 "/Engine/MapTemplates/Materials/BasicTemplateMaterial.BasicTemplateMaterial")
      (Rendering|Material|SetMaterial (Variables|Default|GetCube1) 0 "/Engine/EditorMaterials/Camera/CineMat.CineMat")
      (else
        (Rendering|Material|SetMaterial _cube 0 "/Engine/EditorMaterials/Camera/CineMat.CineMat")))))

(event Custom|SpawnSpider
  (if (Variables|Default|GetIsClaimed)
    (bind _returnvalue (Game|SpawnActorfromClass "/Game/Blueprints/Spider/BP_Spider.BP_Spider_C" (Transformation|GetWorldTransform (Variables|Default|GetArrow)) "Undefined" 0 0))
    (else
      (Actor|DestroyActor _returnvalue))))

(event Custom|DeactivateClaimed
  (Variables|Default|SetIsClaimed false)
  (CallFunction|SpawnSpider))

(event Custom|ActivateClaimed
  (Variables|Default|SetIsClaimed true)
  (CallFunction|SpawnSpider))

(event EventBeginPlay
  (|CallParentFunction))

(event EventConnectWeb
  (if (not (Variables|Default|GetAlreadyClaimed))
    (CallFunction|ActivateClaimed)
    (Variables|Default|SetAlreadyClaimed true)))

(event EventDeselectSlot
  (bind _cube (Variables|Default|GetCube))
  (|CallParentFunction)
  (if (Variables|Default|GetIsClaimed)
    (Rendering|Material|SetMaterial _cube 0 "/Engine/MapTemplates/Materials/BasicTemplateMaterial.BasicTemplateMaterial")
    (else
      (Rendering|Material|SetMaterial _cube 0 "/Engine/EditorMaterials/Camera/CineMat.CineMat"))))

(event EventClickSlot
  (|CallParentFunction))

(event EventSlotsFull
  (|CallParentFunction)
  (Utilities|FlowControl|Delay 0.3))

(event EventRemoveSlot
  (bind _cube (Variables|Default|GetCube))
  (|CallParentFunction)
  (if (Variables|Default|GetIsClaimed)
    (Rendering|Material|SetMaterial _cube 0 "/Engine/MapTemplates/Materials/BasicTemplateMaterial.BasicTemplateMaterial")
    (else
      (Rendering|Material|SetMaterial _cube 0 "/Engine/EditorMaterials/Camera/CineMat.CineMat"))))

(event EventRemovedWeb
  (|CallParentFunction)
  (if (not (Variables|Default|GetHasWeb))
    (CallFunction|DeactivateClaimed)
    (Variables|Default|SetAlreadyClaimed false)))

(fn ConstructionScript
  (|CallParentFunction)
  (Rendering|Material|SetMaterial (Variables|Default|GetCube) 0 "/Engine/EditorMaterials/Camera/CineMat.CineMat"))