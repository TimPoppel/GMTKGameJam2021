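; Game mode for a turn-based web game, alternating planning and active phases where flies get caught on spider webs.
; Tick waits for moving flies to reach zero, then banks caught flies by flavor into inventory, destroys them and starts planning.
; Box traces along each web stop and flag flies as stuck.
; Activating every den slot sets a target turn for the win screen; a separate event shows the lose screen.
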(event Custom|Start%20Planning
  (Default|CallPlanningModeStart)
  (Development|PrintString "Planning Start")
  (CallFunction|DestroyCaughtFlies)
  (Math|Integer|IncrementInt (Variables|Default|GetTurnNumber)
    (:%20%20
      (bind _asbp_line_controller (Utilities|Casting|CastToBP_LineController (Game|GetPlayerController 0)))
      (Default|UpdateTurnCounter (Variables|/Game/Blueprints/Webs/BP_LineController.BP_LineController_C|GetHudWidget _asbp_line_controller) (Variables|Default|GetTurnNumber))
      (Variables|Default|SetCanNextTurn true)
      (Default|UpdateTurnButton (Variables|/Game/Blueprints/Webs/BP_LineController.BP_LineController_C|GetHudWidget _asbp_line_controller)))))

(event Custom|Start%20Active%20Mode
  (Variables|Default|SetCanNextTurn false)
  (Default|CallActiveModeStart)
  (Development|PrintString "Active Start")
  (Audio|PlaySound2D "/Game/Sounds/FlyInWebCue.FlyInWebCue" 1.0 1.0 0.0 0 0))

(event Custom|LooseTrigger
  ;[1 1 1] Win Lose
  (bind _returnvalue (UserInterface|CreateWidget "/Game/Blueprints/Widgets/WinLoose/LooseScreen.LooseScreen_C" (Game|GetPlayerController 0)))
  (UserInterface|Viewport|AddtoViewport _returnvalue 0))

(event Custom|WinTrigger
  ;[1 1 1] Win Lose
  (bind _returnvalue (UserInterface|CreateWidget "/Game/Blueprints/Widgets/WinLoose/WinScreen.WinScreen_C" (Game|GetPlayerController 0)))
  (UserInterface|Viewport|AddtoViewport _returnvalue 0))

(event Custom|Den%20Activated
  (bind _output_get (Variables|Default|SetActivated%20Den%20Numbers (+ (Variables|Default|GetActivated%20Den%20Numbers) 1)))
  (if (== _output_get (Variables|Default|GetDen%20Number))
    (Variables|Default|SetCheck%20For%20win true)
    (Variables|Default|SetTurn%20to%20Beat (+ (Variables|Default|GetTurnNumber) (Variables|Default|GetTurns%20Needed%20to%20Win%20after%20All%20Dens%20Are%20Unlocked)))))

(event EventBeginPlay
  (bind _outactors (Actor|GetAllActorsOfClass "/Game/Blueprints/Webs/BP_SpiderDenSlot.BP_SpiderDenSlot_C"))
  (Variables|Default|SetDen%20Number (Utilities|Array|Length _outactors)))

(event EventTick
  (params (DeltaSeconds :type Float%20%28single-precision%29))
  (if (Variables|Default|GetGame%20Start)
    (if (== (Variables|Default|GetMoving%20Flies) 0)
      (Utilities|FlowControl|DoOnce false :!label _label
        (:Completed
          (Default|CallRoundEnd)
          (Development|PrintString "Round Over")
          (if (Variables|Default|GetCheck%20For%20win)
            (if (== (Variables|Default|GetTurn%20to%20Beat) (Variables|Default|GetTurnNumber))
              (CallFunction|WinTrigger)
              (else
                (bind (_number_sweet _number_sour _number_spicy _number_null) (CallFunction|GetNumberOfCaughtFlies :!label _label_2))
                (Default|AddFlies (Variables|Default|GetInventory%20Reference) _number_sweet _number_sour _number_spicy _number_null)
                (CallFunction|StartPlanning)))
            (else
              (goto _label_2)))))
      (else
        (goto _label Reset)))))

(fn ConstructionScript)

(fn FlyChange
  (params (NewParam :type Integer))
  (bind _output_get (Variables|Default|SetMoving%20Flies (+ NewParam (Variables|Default|GetMoving%20Flies))))
  (Development|PrintString (Utilities|String|ToString(Integer) _output_get)))

(fn StopFliesonWeb
  (bind _outactors (Actor|GetAllActorsOfClass "/Game/Blueprints/Webs/BP_Web.BP_Web_C"))
  (for _array_element _outactors
    (bind _outhits (Class|KismetSystemLibrary|BoxTraceMulti (Variables|/Game/Blueprints/Webs/BP_Web.BP_Web_C|GetStartPos _array_element) (Variables|/Game/Blueprints/Webs/BP_Web.BP_Web_C|GetEndPos _array_element) "6.000000,15.000000,6.000000" "0, 0, 0" "TraceTypeQuery1" false 0 "ForOneFrame" true))
    (for _array_element_2 _outhits
      (bind _asbp_fly (Utilities|Casting|CastToBP_Fly (.hitactor _array_element_2)))
      (Default|StopMoving _asbp_fly)
      (Variables|/Game/Blueprints/Flies/BP_Fly.BP_Fly_C|SetStuck%20on%20web _asbp_fly true))))

(fn DestroyCaughtFlies
  (bind _outactors (Actor|GetAllActorsOfClass "/Game/Blueprints/Flies/BP_Fly.BP_Fly_C"))
  (for _array_element _outactors
    (if (Variables|/Game/Blueprints/Flies/BP_Fly.BP_Fly_C|GetStuck%20on%20web _array_element)
      (Utilities|Array|Add (LocalVariables|GetFlies%20to%20Kill) _array_element)))
  (Actor|DestroyActor (LocalVariables|GetFlies%20to%20Kill)))

(fn GetNumberOfCaughtFlies
  (bind _outactors (Actor|GetAllActorsOfClass "/Game/Blueprints/Flies/BP_Fly.BP_Fly_C"))
  (for _array_element _outactors
    (if (Variables|/Game/Blueprints/Flies/BP_Fly.BP_Fly_C|GetStuck%20on%20web _array_element)
      (switch Utilities|FlowControl|Switch|SwitchonFlavorEnumerator (Variables|/Game/Blueprints/Flies/BP_Fly.BP_Fly_C|GetFlavor _array_element)
        (:NewEnumerator0
          (LocalVariables|SetNumber%20of%20Sweet%20flies (+ (LocalVariables|GetNumber%20of%20Sweet%20flies) 1)))
        (:NewEnumerator1
          (LocalVariables|SetNumber%20of%20Sour%20flies (+ (LocalVariables|GetNumber%20of%20Sour%20flies) 1)))
        (:NewEnumerator2
          (LocalVariables|SetNumber%20of%20Spicy%20flies (+ (LocalVariables|GetNumber%20of%20Spicy%20flies) 1)))
        (:NewEnumerator3
          (LocalVariables|SetNumber%20of%20Null%20flies (+ (LocalVariables|GetNumber%20of%20Null%20flies) 1))))))
  (return (LocalVariables|GetNumber%20of%20Sweet%20flies) (LocalVariables|GetNumber%20of%20Sour%20flies) (LocalVariables|GetNumber%20of%20Spicy%20flies) (LocalVariables|GetNumber%20of%20Null%20flies)))