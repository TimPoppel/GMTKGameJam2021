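; BP_Web is a temporary web strand stretched between two locations that expires after a countdown of planning phases.
; Its construction script reads both endpoints from BP_LineGamemode's WebLocations, then fits the spline and a single spline mesh between them.
; Each planning mode start event from the game mode decrements WebCountdown.
; On expiry it removes itself from each BP_LineSlot's ConnectedWebs, calls RemovedWeb on those slots and destroys itself.
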(event Custom|Countdown
  (bind _result (Math|Integer|DecrementInt (Variables|Default|GetWebCountdown))
    (:%20%20
      (if (< _result 1)
        (bind _outactors (Actor|GetAllActorsOfClass "/Game/Blueprints/Webs/BP_LineSlot.BP_LineSlot_C"))
        (for _array_element _outactors
          (if (Utilities|Array|ContainsItem (Variables|/Game/Blueprints/Webs/BP_LineSlot.BP_LineSlot_C|GetConnectedWebs _array_element) self)
            (Utilities|Array|RemoveItem (Variables|/Game/Blueprints/Webs/BP_LineSlot.BP_LineSlot_C|GetConnectedWebs _array_element) self)
            (Default|RemovedWeb _array_element)))
        (Actor|DestroyActor)))))

(event EventBeginPlay
  (bind _asbp_line_gamemode (Utilities|Casting|CastToBP_LineGamemode (Game|GetGameMode)))
  (EventDispatchers|BindEventtoPlanningModeStart _asbp_line_gamemode (delegate Custom|Countdown)))

(fn ConstructionScript
  (bind _returnvalue (Game|GetGameMode))
  (bind _returnvalue_2 (Game|GetGameMode))
  (bind _splinemesh (Variables|Default|GetSplineMesh))
  (bind _asbp_line_gamemode (Utilities|Casting|CastToBP_LineGamemode _returnvalue))
  (bind _asbp_line_gamemode_2 (Utilities|Casting|CastToBP_LineGamemode _returnvalue_2))
  (bind _weblocations (Variables|/Game/Blueprints/Webs/BP_LineGamemode.BP_LineGamemode_C|GetWebLocations _asbp_line_gamemode))
  (bind _weblocations_2 (Variables|/Game/Blueprints/Webs/BP_LineGamemode.BP_LineGamemode_C|GetWebLocations _asbp_line_gamemode_2))
  (Spline|SetLocationatSplinePoint (Variables|Default|GetSpline) 0 (Utilities|Array|Get(acopy) _weblocations_2) "World" true)
  (Spline|SetLocationatSplinePoint (Variables|Default|GetSpline) 1 (Utilities|Array|Get(acopy) _weblocations_2 1) "World" true)
  (for _index (range 0 (- (Spline|GetNumberOfSplinePoints (Variables|Default|GetSpline)) 1))
    (SplineMesh|SetForwardAxis _splinemesh "Z" true)
    (SplineMesh|SetStartandEnd _splinemesh (Utilities|Array|Get(acopy) _weblocations) (Spline|GetTangentatSplinePoint (Variables|Default|GetSpline) _index "Local") (Utilities|Array|Get(acopy) _weblocations 1) (Spline|GetTangentatSplinePoint (Variables|Default|GetSpline) (+ _index 1) "Local") true :!class /Script/Engine.SplineMeshComponent)))