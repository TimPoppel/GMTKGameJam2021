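; Player controller for web building: left-clicking two points on line slots or existing webs strings a web between them.
; Cursor traces store picks in an actor-to-location map, spawning range and click indicators; clicking a pick again deselects it.
; A second pick must be within MaxLength; slot-to-slot links also need an already-connected slot.
; PlaceWeb hands endpoints to BP_LineGamemode, spawns BP_Web, updates slots and spends one string from StringsToUse.
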(event Custom|AddWebString
  (params (Amount%20of%20Strings :type Integer))
  (bind _output_get (Variables|Default|SetStringsToUse (+ Amount%20of%20Strings (Variables|Default|GetStringsToUse)))))

(event EventBeginPlay
  (Variables|Default|SetbShowMouseCursor true)
  (Variables|Default|SetbEnableMouseOverEvents true)
  (Variables|Default|SetbEnableClickEvents true))

(event Input|MouseEvents|LeftMouseButton
  (params (Key :type Key%20Structure :default "None"))
  (bind _self self)
  (bind _hitresult (Game|Player|GetHitResultUnderCursorbyChannel _self "TraceTypeQuery1" true))
  (bind (_bblockinghit _binitialoverlap _time _distance _location _impactpoint _normal _impactnormal _physmat _hitactor) (Collision|BreakHitResult _hitresult))
  (:Pressed
    (if (> (Variables|Default|GetStringsToUse) 0)
      (bind _asbp_line_slot (Utilities|Casting|CastToBP_LineSlot _hitactor)
        (:then
          (Variables|Default|SetClickedSlot _asbp_line_slot)
          (Variables|Default|SetClickedLocation _location)
          (if (Utilities|Map|Contains (Variables|Default|GetActorClickLocation) (Variables|Default|GetClickedSlot))
            (Default|DeselectSlot (.AsBP%20Line%20Slot (Utilities|Casting|CastToBP_LineSlot (Variables|Default|GetClickedSlot))))
            (Utilities|Map|Remove (Variables|Default|GetActorClickLocation) (Variables|Default|GetClickedSlot))
            (Actor|DestroyActor (Variables|Default|GetWebRangeIndicator))
            (elif (<= (Utilities|Map|Length (Variables|Default|GetActorClickLocation)) 1)
              (Utilities|Map|Add (Variables|Default|GetActorClickLocation) (Variables|Default|GetClickedSlot) (Variables|Default|GetClickedLocation))
              (Default|ClickSlot (.AsBP%20Line%20Slot (Utilities|Casting|CastToBP_LineSlot (Variables|Default|GetClickedSlot))))
              (if (<= (Utilities|Map|Length (Variables|Default|GetActorClickLocation)) 1)
                (bind _returnvalue (Game|SpawnActorfromClass "/Game/Blueprints/Webs/BP_WebRange.BP_WebRange_C" (Math|Transform|MakeTransform (Variables|Default|GetClickedLocation) "0, 0, 0" (* "1.000000,1.000000,1.000000" (/ (Variables|Default|GetMaxLength) (Variables|Default|GetStandardRangeIndicator)))) "Undefined" 0 0))
                (Variables|Default|SetWebRangeIndicator _returnvalue)
                (else
                  (bind _outputpin (CallFunction|HasWeb))
                  (if _outputpin
                    (bind _values (Utilities|Map|Values (Variables|Default|GetActorClickLocation)))
                    (if (> (Math|Vector|Distance(Vector) (Utilities|Array|Get(acopy) _values) (Utilities|Array|Get(acopy) _values 1)) (Variables|Default|GetMaxLength))
                      (Default|SlotsFull (.AsBP%20Line%20Slot (Utilities|Casting|CastToBP_LineSlot (Variables|Default|GetClickedSlot))))
                      (Utilities|Map|Remove (Variables|Default|GetActorClickLocation) (Variables|Default|GetClickedSlot))
                      (Development|PrintString "Web is too long")
                      (else
                        (CallFunction|PlaceWeb)
                        (Actor|DestroyActor (Variables|Default|GetWebRangeIndicator))))
                    (else
                      (Development|PrintString "Not connected to the web")
                      (CallFunction|RemoveLineSlots)
                      (Utilities|Map|Clear (Variables|Default|GetActorClickLocation))
                      (Actor|DestroyActor (Variables|Default|GetWebRangeIndicator))))))
              (else
                (Default|SlotsFull (.AsBP%20Line%20Slot (Utilities|Casting|CastToBP_LineSlot (Variables|Default|GetClickedSlot))))))))
        (:CastFailed
          (bind _asbp_web (Utilities|Casting|CastToBP_Web _hitactor)
            (:then
              (Variables|Default|SetClickedSlot _asbp_web)
              (Variables|Default|SetClickedLocation _location)
              (if (Utilities|Map|Contains (Variables|Default|GetActorClickLocation) (Variables|Default|GetClickedSlot))
                (Utilities|Array|RemoveItem (Variables|Default|GetClickIndicators) (Variables|Default|GetClickIndicator))
                (Actor|DestroyActor (Variables|Default|GetClickIndicator))
                (Utilities|Map|Remove (Variables|Default|GetActorClickLocation) (Variables|Default|GetClickedSlot))
                (Actor|DestroyActor (Variables|Default|GetWebRangeIndicator))
                (elif (<= (Utilities|Map|Length (Variables|Default|GetActorClickLocation)) 1)
                  (Utilities|Map|Add (Variables|Default|GetActorClickLocation) (Variables|Default|GetClickedSlot) (Variables|Default|GetClickedLocation))
                  (bind _returnvalue_2 (Game|SpawnActorfromClass "/Game/Blueprints/Webs/ClickIndicator.ClickIndicator_C" (Math|Transform|MakeTransform (Variables|Default|GetClickedLocation) "0, 0, 0" "1,1,1") "Undefined" 0 0))
                  (bind _output_get (Variables|Default|SetClickIndicator _returnvalue_2))
                  (Utilities|Array|Add (Variables|Default|GetClickIndicators) _output_get)
                  (if (<= (Utilities|Map|Length (Variables|Default|GetActorClickLocation)) 1)
                    (bind _returnvalue_3 (Game|SpawnActorfromClass "/Game/Blueprints/Webs/BP_WebRange.BP_WebRange_C" (Math|Transform|MakeTransform (Variables|Default|GetClickedLocation) "0, 0, 0" (* "1.000000,1.000000,1.000000" (/ (Variables|Default|GetMaxLength) (Variables|Default|GetStandardRangeIndicator)))) "Undefined" 0 0))
                    (Variables|Default|SetWebRangeIndicator _returnvalue_3)
                    (else
                      (bind _values_2 (Utilities|Map|Values (Variables|Default|GetActorClickLocation)))
                      (if (> (Math|Vector|Distance(Vector) (Utilities|Array|Get(acopy) _values_2) (Utilities|Array|Get(acopy) _values_2 1)) (Variables|Default|GetMaxLength))
                        (Default|OutOfRange (Variables|Default|GetClickIndicator))
                        (Utilities|Map|Remove (Variables|Default|GetActorClickLocation) (Variables|Default|GetClickedSlot))
                        (Development|PrintString "Web is too long")
                        (else
                          (CallFunction|PlaceWeb)
                          (Actor|DestroyActor (Variables|Default|GetWebRangeIndicator)))))))))
            (:CastFailed
              (bind _asclick_indicator (Utilities|Casting|CastToClickIndicator _hitactor))
              (if (== _asclick_indicator (Variables|Default|GetClickIndicator))
                (if (not (Variables|/Game/Blueprints/Webs/ClickIndicator.ClickIndicator_C|GetIsPlaced (Variables|Default|GetClickIndicator)))
                  (Utilities|Array|RemoveItem (Variables|Default|GetClickIndicators) (Variables|Default|GetClickIndicator))
                  (Actor|DestroyActor (Variables|Default|GetClickIndicator))
                  (Utilities|Map|Remove (Variables|Default|GetActorClickLocation) (Variables|Default|GetClickedSlot))
                  (Actor|DestroyActor (Variables|Default|GetWebRangeIndicator)))))))))))

(fn ConstructionScript)

(fn PlaceWeb
  (bind _clickindicators (Variables|Default|GetClickIndicators))
  (bind _clickindicators_2 (Variables|Default|GetClickIndicators))
  (bind _output (Utilities|Array|Get(acopy) _clickindicators 1))
  (bind _output_2 (Utilities|Array|Get(acopy) _clickindicators_2))
  (bind _values (Utilities|Map|Values (Variables|Default|GetActorClickLocation)))
  (bind _asbp_line_gamemode (Utilities|Casting|CastToBP_LineGamemode (Game|GetGameMode)))
  (Variables|/Game/Blueprints/Webs/BP_LineGamemode.BP_LineGamemode_C|SetWebLocations _asbp_line_gamemode _values)
  (bind _returnvalue (Game|SpawnActorfromClass "/Game/Blueprints/Webs/BP_Web.BP_Web_C" (Math|Transform|MakeTransform "0, 0, 0" "0, 0, 0" "1,1,1") "Undefined" 0 0))
  (LocalVariables|SetSpawnedWeb _returnvalue)
  (bind _keys (Utilities|Map|Keys (Variables|Default|GetActorClickLocation)))
  (if (.bSuccess (Utilities|Casting|CastToBP_LineSlot (Utilities|Array|Get(acopy) _keys)))
    (Default|DeselectSlot (.AsBP%20Line%20Slot (Utilities|Casting|CastToBP_LineSlot (Utilities|Array|Get(acopy) _keys))))
    (Utilities|Array|Add (Variables|/Game/Blueprints/Webs/BP_LineSlot.BP_LineSlot_C|GetConnectedWebs (.AsBP%20Line%20Slot (Utilities|Casting|CastToBP_LineSlot (Utilities|Array|Get(acopy) _keys)))) (LocalVariables|GetSpawnedWeb)))
  (if (.bSuccess (Utilities|Casting|CastToBP_LineSlot (Utilities|Array|Get(acopy) _keys 1)))
    (Default|DeselectSlot (.AsBP%20Line%20Slot (Utilities|Casting|CastToBP_LineSlot (Utilities|Array|Get(acopy) _keys 1))))
    (Utilities|Array|Add (Variables|/Game/Blueprints/Webs/BP_LineSlot.BP_LineSlot_C|GetConnectedWebs (.AsBP%20Line%20Slot (Utilities|Casting|CastToBP_LineSlot (Utilities|Array|Get(acopy) _keys 1)))) (LocalVariables|GetSpawnedWeb)))
  (bind _keys_2 (Utilities|Map|Keys (Variables|Default|GetActorClickLocation)))
  (for _array_element _keys_2
    (bind _asbp_line_slot (Utilities|Casting|CastToBP_LineSlot _array_element))
    (if (> (Utilities|Array|Length (Variables|/Game/Blueprints/Webs/BP_LineSlot.BP_LineSlot_C|GetConnectedWebs _asbp_line_slot)) 0)
      (Variables|/Game/Blueprints/Webs/BP_LineSlot.BP_LineSlot_C|SetHasWeb _asbp_line_slot true)
      (Default|ConnectWeb _asbp_line_slot)))
  (Utilities|IsValid _output_2
    (:Is%20Valid
      (Default|Deselect _output_2))
    (:Is%20Not%20Valid
      _))
  (Utilities|IsValid _output
    (:Is%20Valid
      (Default|Deselect _output))
    (:Is%20Not%20Valid
      _))
  (Utilities|Map|Clear (Variables|Default|GetActorClickLocation))
  (Utilities|Array|Clear (Variables|Default|GetClickIndicators))
  (Math|Integer|DecrementInt (Variables|Default|GetStringsToUse)))

(fn HasWeb
  (LocalVariables|SetIsWeb false)
  (bind _keys (Utilities|Map|Keys (Variables|Default|GetActorClickLocation)))
  (Utilities|IsValid (.AsBP%20Line%20Slot (Utilities|Casting|CastToBP_LineSlot (Utilities|Array|Get(acopy) _keys)))
    (:Is%20Valid
      (Utilities|IsValid (.AsBP%20Line%20Slot (Utilities|Casting|CastToBP_LineSlot (Utilities|Array|Get(acopy) _keys 1)))
        (:Is%20Valid
          (LocalVariables|SetConnected (or (or (Variables|/Game/Blueprints/Webs/BP_LineSlot.BP_LineSlot_C|GetHasWeb (.AsBP%20Line%20Slot (Utilities|Casting|CastToBP_LineSlot (Utilities|Array|Get(acopy) _keys)))) (Variables|/Game/Blueprints/Webs/BP_LineSlot.BP_LineSlot_C|GetHasWeb (.AsBP%20Line%20Slot (Utilities|Casting|CastToBP_LineSlot (Utilities|Array|Get(acopy) _keys 1))))) (LocalVariables|GetConnected))))
        (:Is%20Not%20Valid
          (LocalVariables|SetConnected true))))
    (:Is%20Not%20Valid
      (LocalVariables|SetConnected true)))
  (return (LocalVariables|GetConnected)))

(fn RemoveLineSlots
  (bind _keys (Utilities|Map|Keys (Variables|Default|GetActorClickLocation)))
  (if (.bSuccess (Utilities|Casting|CastToBP_LineSlot (Utilities|Array|Get(acopy) _keys)))
    (Default|RemoveSlot (.AsBP%20Line%20Slot (Utilities|Casting|CastToBP_LineSlot (Utilities|Array|Get(acopy) _keys)))))
  (if (.bSuccess (Utilities|Casting|CastToBP_LineSlot (Utilities|Array|Get(acopy) _keys 1)))
    (Default|RemoveSlot (.AsBP%20Line%20Slot (Utilities|Casting|CastToBP_LineSlot (Utilities|Array|Get(acopy) _keys 1))))))