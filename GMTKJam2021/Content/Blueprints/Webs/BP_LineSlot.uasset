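; BP_LineSlot is a cube slot for webs that shows hover, selection and rejection feedback by swapping materials.
; Cursor hover changes the material only while unselected, and events toggle selection, reset the slot or briefly flash red when slots are full.
; RemovedWeb updates HasWeb from the ConnectedWebs count, and the construction script applies a separate material when HasWeb is set.
; The cube's click handler and ConnectWeb are empty.
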(event OnBeginCursorOver(Cube)
  (params (TouchedComponent :type Primitive%20Component%20Object%20Reference))
  (if (not (Variables|Default|GetIsSelected))
    (Rendering|Material|SetMaterial (Variables|Default|GetCube) 0 "/DatasmithContent/Materials/Arealight.Arealight")))

(event OnEndCursorOver(Cube)
  (params (TouchedComponent :type Primitive%20Component%20Object%20Reference))
  (if (not (Variables|Default|GetIsSelected))
    (Rendering|Material|SetMaterial (Variables|Default|GetCube) 0 "/Engine/MapTemplates/Materials/BasicTemplateMaterial.BasicTemplateMaterial")))

(event OnClicked(Cube)
  (params (TouchedComponent :type Primitive%20Component%20Object%20Reference) (ButtonPressed :type Key%20Structure :default "None")))

(event Custom|ClickSlot
  (Variables|Default|SetIsSelected true)
  (Rendering|Material|SetMaterial (Variables|Default|GetCube) 0 "/AnimationSharing/AnimSharingGreen.AnimSharingGreen"))

(event Custom|SlotsFull
  (Rendering|Material|SetMaterial (Variables|Default|GetCube) 0 "/AnimationSharing/AnimSharingRed.AnimSharingRed")
  (Utilities|FlowControl|Delay 0.2)
  (Rendering|Material|SetMaterial (Variables|Default|GetCube) 0 "/Engine/MapTemplates/Materials/BasicTemplateMaterial.BasicTemplateMaterial"))

(event Custom|DeselectSlot
  (Variables|Default|SetIsSelected false)
  (Rendering|Material|SetMaterial (Variables|Default|GetCube) 0 "/DatasmithContent/Materials/Arealight.Arealight"))

(event Custom|RemoveSlot
  (Rendering|Material|SetMaterial (Variables|Default|GetCube) 0 "/Engine/MapTemplates/Materials/BasicTemplateMaterial.BasicTemplateMaterial"))

(event Custom|RemovedWeb
  (if (> (Utilities|Array|Length (Variables|Default|GetConnectedWebs)) 0)
    (Variables|Default|SetHasWeb true)
    (else
      (Variables|Default|SetHasWeb false))))

(event Custom|ConnectWeb)

(event EventBeginPlay)

(event Collision|EventActorBeginOverlap
  (params (OtherActor :type Actor%20Object%20Reference)))

(fn ConstructionScript
  (if (Variables|Default|GetHasWeb)
    (Rendering|Material|SetMaterial (Variables|Default|GetCube) 0 "/DatasmithContent/Materials/AliasMaster.AliasMaster")))