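; BP_WallLoL is a wall actor that slides along world Y between StartY and EndY in response to BP_LineGamemode round events.
; On RoundEnd, if Active, a FlipFlop alternates playing and reversing a timeline that lerps the root's position.
; A start-closed DoOnce, reopened by ActiveModeStart, limits it to one move per reset.
; The construction script applies Material0 to its cube.
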(event Custom|Move%20Wall
  (bind _defaultsceneroot (Variables|Default|GetDefaultSceneRoot))
  (bind _returnvalue (Transformation|GetWorldLocation _defaultsceneroot))
  (if (Variables|Default|GetActive)
    (Utilities|FlowControl|DoOnce true
      (:Completed
        (Utilities|FlowControl|FlipFlop
          (:A
            (bind _newtrack_0 (Timeline|Timeline_0 PlayFromStart)
              (:Update
                (Transformation|SetWorldLocation _defaultsceneroot (Math|Vector|MakeVector (.x _returnvalue) (Math|Float|Lerp (Variables|Default|GetStart%20Y) (Variables|Default|GetEnd%20Y) _newtrack_0) (.z _returnvalue)) false false))))
          (:B
            (Timeline|Timeline_0 ReverseFromEnd)))))))

(event Custom|Reset
  (bind _defaultsceneroot (Variables|Default|GetDefaultSceneRoot))
  (bind _returnvalue (Transformation|GetWorldLocation _defaultsceneroot))
  (Utilities|FlowControl|DoOnce true) ; enters at Reset
)

(event EventBeginPlay
  (bind _asbp_line_gamemode (Utilities|Casting|CastToBP_LineGamemode (Game|GetGameMode)))
  (Utilities|FlowControl|Sequence
    (:then_0
      (EventDispatchers|BindEventtoRoundEnd _asbp_line_gamemode (delegate Custom|Move%20Wall)))
    (:then_1
      (EventDispatchers|BindEventtoActiveModeStart _asbp_line_gamemode (delegate Custom|Reset)))))

(event Collision|EventActorBeginOverlap
  (params (OtherActor :type Actor%20Object%20Reference)))

(event EventTick
  (params (DeltaSeconds :type Float%20%28single-precision%29)))

(fn ConstructionScript
  (Rendering|Material|SetMaterial (Variables|Default|GetCube) 0 (Variables|Default|GetMaterial_0)))