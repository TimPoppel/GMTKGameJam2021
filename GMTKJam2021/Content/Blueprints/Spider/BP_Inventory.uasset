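; BP_Inventory tracks the Flies and Strings resources for the spider game.
; A looping timer started on BeginPlay adds a fly at a fixed interval and prints both counts.
; AddString increases Strings, while FeedFlies spends a fly to call GetFed on a given spider, or prints a notice when none remain.
; A timer meant to run FeedFlies automatically is left disconnected.
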(event Custom|AddString
  (params (StringAmount :type Integer))
  (Variables|Default|SetStrings (+ StringAmount (Variables|Default|GetStrings))))

(event Collision|EventActorBeginOverlap
  (params (OtherActor :type Actor%20Object%20Reference)))

(event EventBeginPlay
  (Utilities|Time|SetTimerbyFunctionName 0 "AddFlies" 5.0 true))

(fn ConstructionScript)

(fn AddFlies
  (bind _output_get (Variables|Default|SetFlies (+ (Variables|Default|GetFlies) 1)))
  (Development|PrintString (Utilities|String|ToString(Integer) _output_get))
  (Development|PrintString (Utilities|String|ToString(Integer) (Variables|Default|GetStrings))))

(fn FeedFlies
  (params (SpiderTarget :type BP%20Spider%20Object%20Reference))
  (if (<= (Variables|Default|GetFlies) 0)
    (Development|PrintString "no flies")
    (else
      (Default|GetFed SpiderTarget 1)
      (Variables|Default|SetFlies (- (Variables|Default|GetFlies) 1)))))