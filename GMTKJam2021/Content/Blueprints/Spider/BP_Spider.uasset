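; BP_Spider is a clickable spider that the player feeds flies from BP_Inventory to earn web string.
; Clicking its sphere requests feeding, and GetFed weighs the flavor against likes and dislikes, then checks survival and happiness thresholds.
; A happy spider spends flies and adds string to BP_LineController.
; An underfed one is flagged for damage, so TakeDamage costs a life and destroys it when none remain.
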(event OnClicked(Sphere)
  (params (TouchedComponent :type Primitive%20Component%20Object%20Reference) (ButtonPressed :type Key%20Structure :default "None"))
  (bind _returnvalue (Actor|GetActorOfClass "/Game/Blueprints/Spider/BP_Inventory.BP_Inventory_C"))
  (Default|FeedFlies _returnvalue self))

(event Custom|ProduceString
  ;[1 1 1] Give string to the player
  (bind _asbp_line_controller (Utilities|Casting|CastToBP_LineController (Game|GetPlayerController 0)))
  (Default|AddWebString _asbp_line_controller (Variables|Default|GetString)))

(event Custom|SetHappy
  (Variables|Default|SetIsHappy true)
  (Development|PrintString "I am Happy :)")
  (CallFunction|ProduceString)
  (Variables|Default|SetFliesGotten (- (Variables|Default|GetFliesGotten) (Variables|Default|GetFliesneed)))
  (Variables|Default|SetIsHappy false)
  (Variables|Default|SetWillTakeDmg false))

(event Custom|GetFed
  (params (FliesAmount :type Integer) (Flavor :type FlavorEnumerator%20Enum :default "NewEnumerator0"))
  (if (Utilities|Enum|Equal(Enum) Flavor (Variables|Default|GetLikes))
    (Variables|Default|SetFliesGotten (+ FliesAmount (Variables|Default|GetFliesGottenLiked)))
    (if (>= (Variables|Default|GetFliesGotten) (Variables|Default|GetFliesToStayAlive)) :!label _label
      (Variables|Default|SetWillTakeDmg false)
      (if (>= (Variables|Default|GetFliesGotten) (Variables|Default|GetFliesneed))
        (CallFunction|SetHappy)
        (else
          (Development|PrintString "I still need more flies :(" :!label _label_2)))
      (else
        (Variables|Default|SetWillTakeDmg true)
        (goto _label_2)))
    (elif (Utilities|Enum|Equal(Enum) Flavor (Variables|Default|GetDislikes))
      (Development|PrintString "yuck")
      (else
        (Variables|Default|SetFliesGotten (+ FliesAmount (Variables|Default|GetFliesGottenNeutral)))
        (goto _label)))))

(event Custom|Take%20Damage
  (if (Variables|Default|GetWillTakeDmg)
    (Math|Integer|DecrementInt (Variables|Default|GetLifes)
      (:%20%20
        (CallFunction|Die)))))

(event Custom|Die
  (if (<= (Variables|Default|GetLifes) 0)
    (Actor|DestroyActor)))

(event EventBeginPlay
  (if (Variables|Default|GetWillTakeDmg)
    (Development|PrintString (Utilities|String|ToString(Integer) (Variables|Default|GetFliesneed)))
    (Development|PrintString "I want flies :(")
    (elif (Variables|Default|GetIsHappy)
      (CallFunction|ProduceString)
      (Variables|Default|SetFliesGotten (- (Variables|Default|GetFliesGotten) (Variables|Default|GetFliesneed)))
      (Variables|Default|SetIsHappy false)
      (else
        (Variables|Default|SetFliesGotten (- (Variables|Default|GetFliesGotten) (Variables|Default|GetFliesToStayAlive)))))))

(fn ConstructionScript)