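; BP_FlyWall is a box-shaped wall that can stop flies which run into it.
; When an actor begins overlapping while StopThem is on, a BP_Fly is told to stop moving and check for death.
; A ToggleStopThem event uses a FlipFlop to switch that blocking on and off.
; The construction script sizes the box from ExtendUpDown and ExtendRightLeft, keeping a fixed thickness.
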(event Custom|Toggle%20Stop%20Them
  (bind _isa (Utilities|FlowControl|FlipFlop)
    (:A
      _)
    (:B
      _))
  (Variables|Default|SetStopThem (not _isa)))

(event EventBeginPlay)

(event Collision|EventActorBeginOverlap
  (params (OtherActor :type Actor%20Object%20Reference))
  (bind _asbp_fly (Utilities|Casting|CastToBP_Fly OtherActor))
  (if (Variables|Default|GetStopThem)
    (Default|StopMoving _asbp_fly)
    (Default|CheckDeath _asbp_fly)))

(event EventTick
  (params (DeltaSeconds :type Float%20%28single-precision%29)))

(fn ConstructionScript
  (Components|Box|SetBoxExtent (Variables|Default|GetBox) (Math|Vector|MakeVector (Variables|Default|GetExtend%20UpDown) 5e+01 (Variables|Default|GetExtend%20RightLeft)) true))