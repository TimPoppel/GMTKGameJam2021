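; BP_FlyTarget is a fly spawner that registers itself with BP_LineGamemode and spawns a batch of flies when the round-end event fires.
; Each batch uses a FlipFlop to alternate sides along Y at WallDistance, turning spawn yaw 180 degrees each time.
; Flies appear at random X/Z points within Extend, which also sizes the box, and get a random flavor plus optionally randomized readability.
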(event Custom|Spawn%20x%20Flies
  (params (Number :type Integer))
  (bind _defaultsceneroot (Variables|Default|GetDefaultSceneRoot))
  (bind _extend (Variables|Default|GetExtend))
  (bind _returnvalue (Transformation|GetWorldLocation _defaultsceneroot))
  (bind _isa (Utilities|FlowControl|FlipFlop)
    (:A
      _)
    (:B
      _))
  (Variables|Default|SetSpawn%20distance (* (- 1 (* (Math|Conversions|ToInteger(Boolean) _isa) 2)) (Variables|Default|GetWallDistance)))
  (Variables|Default|SetSpawn%20Transform%20Rotation%20Z%20%28Yaw%29 (+ (Variables|Default|GetSpawn%20Transform%20Rotation%20Z%20%28Yaw%29) 1.8e+02))
  (for _index (range 1 Number)
    ;[1 1 1] Spawn Fly
    (bind _returnvalue_2 (Game|SpawnActorfromClass "/Game/Blueprints/Flies/BP_Fly.BP_Fly_C" (Math|Transform|MakeTransform (Math|Vector|MakeVector (+ (.x _returnvalue) (Math|Random|RandomFloatinRange (* -1 _extend) _extend)) (+ (.y _returnvalue) (Variables|Default|GetSpawn%20distance)) (+ (Math|Random|RandomFloatinRange (* -1 _extend) _extend) (.z _returnvalue))) (Math|Rotator|MakeRotator 0.0 0.0 (Variables|Default|GetSpawn%20Transform%20Rotation%20Z%20%28Yaw%29)) "1,1,1") "AlwaysSpawn" 0 0))
    (Default|Initialize _returnvalue_2)
    (Default|SetFlavor _returnvalue_2 (.OutItem (Utilities|Array|Random (Variables|Default|GetFlavors))))
    (if (Variables|Default|GetRandomReadability)
      (Variables|/Game/Blueprints/Flies/BP_Fly.BP_Fly_C|SetReadable _returnvalue_2 (Math|Random|RandomBoolwithWeight (Variables|Default|GetReadable%20Chance))))))

(event Custom|Debug%20Spawn%20Group%20Flies
  (CallFunction|SpawnXFlies (Variables|Default|GetTo%20Spawn)))

(event EventBeginPlay
  (Utilities|FlowControl|Sequence
    (:then_0
      (bind _asbp_line_gamemode (Utilities|Casting|CastToBP_LineGamemode (Game|GetGameMode)))
      (Variables|/Game/Blueprints/Webs/BP_LineGamemode.BP_LineGamemode_C|SetFlyTargetReference _asbp_line_gamemode self)
      (EventDispatchers|BindEventtoRoundEnd _asbp_line_gamemode (delegate Custom|Debug%20Spawn%20Group%20Flies)))))

(event Collision|EventActorBeginOverlap
  (params (OtherActor :type Actor%20Object%20Reference)))

(event EventTick
  (params (DeltaSeconds :type Float%20%28single-precision%29)))

(fn ConstructionScript
  (bind _extend (Variables|Default|GetExtend))
  (Components|Box|SetBoxExtent (Variables|Default|GetBox) (Math|Vector|MakeVector _extend 1.0 _extend) true))