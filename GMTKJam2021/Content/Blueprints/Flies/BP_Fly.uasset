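; Fly actor for a turn-based game that follows the BP_LineGamemode planning and active phases.
; In planning, it picks a random point around the gamemode's FlyTarget in the XZ plane, stores the direction and spawns a debug sphere there.
; In active mode, a looping timer steps it along that direction while it reports its movement to the gamemode.
; StopMoving clears the timer, and CheckDeath destroys the fly after enough moves.
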(event OnComponentBeginOverlap(Sphere)
  (params (OverlappedComponent :type Primitive%20Component%20Object%20Reference) (OtherActor :type Actor%20Object%20Reference) (OtherComp :type Primitive%20Component%20Object%20Reference) (OtherBodyIndex :type Integer) (bFromSweep :type Boolean) (SweepResult :type Hit%20Result%20Structure%20%28by%20ref%29))
  (Development|PrintString (Utilities|GetDisplayName OtherActor)))

(event Custom|Find%20Move%20Direction%20Normal
  (params (Target :type Vector))
  ;[1 1 1] Find Move Direction Vector
  (Variables|Default|SetOut%20Hit%20Normal (Math|Vector|Normalize (Math|Vector|GetUnitDirection(Vector) (Transformation|GetWorldLocation (Variables|Default|GetDefaultSceneRoot)) Target))))

(event Custom|Move
  (bind _defaultsceneroot (Variables|Default|GetDefaultSceneRoot))
  ;[1 1 1] Movement
  (Transformation|SetWorldLocation _defaultsceneroot (+ (Transformation|GetWorldLocation _defaultsceneroot) (* (Variables|Default|GetOut%20Hit%20Normal) (Variables|Default|GetSpeed))) false false))

(event Custom|Start%20Moving
  ;[1 1 1] Movement
  (Default|MovingFlyChange (Variables|Default|GetAs%20BP%20Line%20Gamemode) 1)
  (Variables|Default|SetMove%20Count (+ (Variables|Default|GetMove%20Count) 1.0))
  (bind _returnvalue (Utilities|Time|SetTimerbyEvent (delegate Custom|Move) 0.01 true))
  (Variables|Default|SetMovement%20Loop _returnvalue))

(event Custom|Initialize
  ;[1 1 1] Initialize
  (Utilities|FlowControl|Sequence
    (:then_0
      (Variables|Default|SetFlyTarget (Variables|/Game/Blueprints/Webs/BP_LineGamemode.BP_LineGamemode_C|GetFlyTargetReference (Variables|Default|GetAs%20BP%20Line%20Gamemode))))))

(event Custom|Turn%20Initialization
  ;[1 1 1] Turn Initialization
  (bind _target (CallFunction|FindRandomTarget (Transformation|GetWorldLocation (Variables|/Game/Blueprints/Flies/BP_FlyTarget.BP_FlyTarget_C|GetDefaultSceneRoot (Variables|Default|GetFlyTarget)))))
  (Utilities|FlowControl|Sequence
    (:then_0
      (CallFunction|FindMoveDirectionNormal _target))
    (:then_1
      (CallFunction|CreateVisualIndicator _target))))

(event Custom|Stop%20Moving
  ;[1 1 1] Stop Moving
  (Utilities|Time|ClearandInvalidateTimerbyHandle (Variables|Default|GetMovement%20Loop))
  (Default|MovingFlyChange (Variables|Default|GetAs%20BP%20Line%20Gamemode) -1))

(event Custom|Check%20Death
  ;[1 1 1] Check Death
  (if (>= (Variables|Default|GetMove%20Count) (Variables|Default|GetMove%20To%20Die))
    (Actor|DestroyActor)))

(event EventBeginPlay
  (bind _asbp_line_gamemode (Utilities|Casting|CastToBP_LineGamemode (Game|GetGameMode)))
  (bind _output_get (Variables|Default|SetAs%20BP%20Line%20Gamemode _asbp_line_gamemode))
  (EventDispatchers|BindEventtoPlanningModeStart _output_get (delegate Custom|Turn%20Initialization))
  (EventDispatchers|BindEventtoActiveModeStart _output_get (delegate Custom|Start%20Moving)))

(event Collision|EventActorBeginOverlap
  (params (OtherActor :type Actor%20Object%20Reference)))

(event EventTick
  (params (DeltaSeconds :type Float%20%28single-precision%29)))

(fn ConstructionScript)

(fn FindRandomTarget
  (params (Center :type Vector))
  (bind _flytarget (Variables|Default|GetFlyTarget))
  (bind _extend (Variables|/Game/Blueprints/Flies/BP_FlyTarget.BP_FlyTarget_C|GetExtend _flytarget))
  (bind _defaultsceneroot (Variables|/Game/Blueprints/Flies/BP_FlyTarget.BP_FlyTarget_C|GetDefaultSceneRoot _flytarget))
  (bind _returnvalue (Transformation|GetWorldLocation _defaultsceneroot))
  (return (Math|Vector|MakeVector (+ (.x _returnvalue) (Math|Random|RandomFloatinRange (* -1 _extend) _extend)) (.y _returnvalue) (+ (Math|Random|RandomFloatinRange (* -1 _extend) _extend) (.z _returnvalue)))))

(fn CreateVisualIndicator
  (params (Location :type Vector))
  (Game|SpawnActorfromClass "/Game/Developers/NianCunahawk/Collections/DebugSphere.DebugSphere_C" (Math|Transform|MakeTransform Location "0, 0, 0" "1,1,1") "AlwaysSpawn" 0 0))